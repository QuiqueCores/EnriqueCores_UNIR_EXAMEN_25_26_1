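; BP_FloorButton is a floor button with a hieroglyph mesh that the player toggles on and off by interacting while standing on it.
; At BeginPlay it binds to the player character's OnInteractPressed event, while a box collider tracks whether the actor tagged Player is inside.
; Actionate flips the state when the player is inside, swaps between on and off emissive materials, and broadcasts OnFloorButtonActionated.
; IsActionated exposes the current state.
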(event `self.ReceiveBeginPlay`
  ; Material inicial (apagado)
  (`PrimitiveComponent.SetMaterial` (`self.SM_hieroglyph_007`) 0 "/Game/00_Examen_UNIR/M_Emission_Btn_Off.M_Emission_Btn_Off")
  ; Guardar referencia a player
  (bind _asbp_third_person_character_examen (cast `/Game/00_Examen_UNIR/BP_ThirdPersonCharacterExamen` (`GameplayStatics.GetPlayerCharacter` 0)))
  (bind _output_get (set `self.PlayerRef` _asbp_third_person_character_examen))
  ; Observar evento interacción del player
  (add `/Game/00_Examen_UNIR/BP_ThirdPersonCharacterExamen.OnInteractPressed` _output_get (delegate `OnInteractPressed_Event`)))

(event `OnInteractPressed_Event`
  ; Observar evento interacción del player
  (`self.Actionate`))

(event `self.BoxCollider.OnComponentBeginOverlap`
  (params (OverlappedComponent :type "PrimitiveComponent Object Reference") (OtherActor :type "Actor Object Reference") (OtherComp :type "PrimitiveComponent Object Reference") (OtherBodyIndex :type Integer) (bFromSweep :type Boolean) (SweepResult :type "HitResult Structure (by ref)"))
  ; Comprobar si el jugador está dentro del collider
  (if (`self.ActorHasTag` OtherActor "Player")
    (set `self.bIsPlayerInside` true)))

(event `self.BoxCollider.OnComponentEndOverlap`
  (params (OverlappedComponent :type "PrimitiveComponent Object Reference") (OtherActor :type "Actor Object Reference") (OtherComp :type "PrimitiveComponent Object Reference") (OtherBodyIndex :type Integer))
  ; Comprobar si el jugador está dentro del collider
  (if (`self.ActorHasTag` OtherActor "Player")
    (set `self.bIsPlayerInside` false)))

(fn `Actionate`
  (returns (Actionated :type Boolean))
  (if (`self.bIsPlayerInside`)
    (bind _output_get (set `self.bIsOn` (not (`self.bIsOn`))))
    (if _output_get
      (`PrimitiveComponent.SetMaterial` (`self.SM_hieroglyph_007`) 0 "/Game/00_Examen_UNIR/M_Emission_Btn_On.M_Emission_Btn_On")
      (else
        (`PrimitiveComponent.SetMaterial` (`self.SM_hieroglyph_007`) 0 "/Game/00_Examen_UNIR/M_Emission_Btn_Off.M_Emission_Btn_Off")))
    (`self.OnFloorButtonActionated`)
    (return _output_get)))

(fn `IsActionated`
  (returns (Actionated :type Boolean))
  (return (`self.bIsOn`)))

(fn `UserConstructionScript`)