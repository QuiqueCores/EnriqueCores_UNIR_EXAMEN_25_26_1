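; BP_Door is a sliding double door that opens only while every floor button in its Buttons array is actuated.
; On BeginPlay it stores both panels' relative positions, binds to each button's actuation event and evaluates the initial state.
; Each button event rechecks all buttons, calling OpenDoor or CloseDoor, each guarded by a DoorIsOpen flag.
; A Timeline lerps the panels apart along local X and reverses to close them.
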(event `self.ReceiveBeginPlay`
  ; Guardar posiciones iniciales de la puerta
  (set `self.DoorRightInitialPos` (`SceneComponent.RelativeLocation` (`self.DoorRight`)))
  (set `self.DoorLeftInitialPos` (`SceneComponent.RelativeLocation` (`self.DoorLeft`)))
  ; Observar eventos de los botones
  (for _array_element (`self.Buttons`)
    (add `/Game/00_Examen_UNIR/BP_FloorButton.OnFloorButtonActionated` _array_element (delegate `OnFloorButtonActionated_Event`))
    (`self.CheckAllButtonPressed`)))

(event `OnFloorButtonActionated_Event`
  ; Observar eventos de los botones
  (`self.CheckAllButtonPressed`))

(event `OpenDoor`
  (if (not (`self.bDoorIsOpen`))
    (set `self.bDoorIsOpen` true)
    ; Mover la puerta con timeline
    (bind (_direction _newtrack_0) (`Timeline|Timeline` :!label _label)
      (:`Update`
        (`SceneComponent.K2_SetRelativeLocation` (`self.DoorRight`) (`KismetMathLibrary.VLerp` (`self.DoorRightInitialPos`) (+ (`self.DoorRightInitialPos`) (80.0 0.0 0.0)) _newtrack_0) false false)
        (`SceneComponent.K2_SetRelativeLocation` (`self.DoorLeft`) (`KismetMathLibrary.VLerp` (`self.DoorLeftInitialPos`) (- (`self.DoorLeftInitialPos`) (80.0 0.0 0.0)) _newtrack_0) false false)))))

(event `CloseDoor`
  (if (`self.bDoorIsOpen`)
    (set `self.bDoorIsOpen` false)
    (goto _label :!via `Reverse`)))

(event `CheckAllButtonPressed`
  ; Comprobar botones
  (set `self.bAllButtonPressed` true)
  (for _array_element (`self.Buttons`)
    (bind _actionated (`/Game/00_Examen_UNIR/BP_FloorButton.IsActionated` _array_element))
    (set `self.bAllButtonPressed` (and _actionated (`self.bAllButtonPressed`))))
  ; Abrir/cerrar puerta
  (if (`self.bAllButtonPressed`)
    (`self.OpenDoor`)
    (else
      (`self.CloseDoor`))))

(fn `UserConstructionScript`)